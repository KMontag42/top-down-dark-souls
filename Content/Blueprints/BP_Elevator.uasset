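; BP_Elevator is an elevator that moves a static mesh along a spline when something overlaps its Collider.
; A timeline samples the spline at constant velocity to set the mesh's world location.
; AtSplineEnd chooses forward or reverse playback and flips when the move finishes, while IsMoving blocks retriggering in transit.
; IsMoving is set before the self-overlap check, so a self overlap leaves it set without moving.
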(event `self.ReceiveTick`
  (params (DeltaSeconds :type "Float (single-precision)")))

(event `self.ReceiveBeginPlay`)

(event `self.Collider.OnComponentBeginOverlap`
  (params (OtherActor :type "Actor Object Reference") (OtherComp :type "PrimitiveComponent Object Reference") (OtherBodyIndex :type Integer) (bFromSweep :type Boolean) (SweepResult :type "HitResult Structure (by ref)"))
  (if (not (`self.IsMoving`))
    (set `self.IsMoving` true)
    (if (!= OtherActor self)
      (if (`self.AtSplineEnd`)
        (bind (_direction _newtrack_6) (`Timeline|Timeline_0` :!via `ReverseFromEnd` :!label _label)
          (:`Update`
            (`SceneComponent.K2_SetWorldLocation` (`self.StaticMesh`) (`SplineComponent.GetLocationAtTime` (`self.Spline`) _newtrack_6 "World" true) false false))
          (:`Finished`
            (set `self.IsMoving` false)
            (set `self.AtSplineEnd` (not (`self.AtSplineEnd`)))))
        (else
          (goto _label :!via `PlayFromStart`))))))

(fn `UserConstructionScript`)